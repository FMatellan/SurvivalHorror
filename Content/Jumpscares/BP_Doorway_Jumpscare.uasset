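; BP_Doorway_Jumpscare is a jumpscare actor that slides a mannequin to a set endpoint, then removes itself.
; Once the CalledJumpscare flag is true, Tick moves Mannequin toward Endpoint at constant speed using VInterpToConstant, without sweeping.
; The actor destroys itself when the mannequin reaches the endpoint within a small tolerance.
; Nothing in this graph sets the flag.
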(event `self.ReceiveTick`
  (params (DeltaSeconds :type "Float (single-precision)"))
  (if (`self.calledJumpscare`)
    (`SceneComponent.K2_SetWorldLocation` (`self.Mannequin`) (`KismetMathLibrary.VInterpTo_Constant` (`SceneComponent.K2_GetComponentLocation` (`self.Mannequin`)) (`SceneComponent.K2_GetComponentLocation` (`self.Endpoint`)) DeltaSeconds 300.0) false false)
    (if (== (`SceneComponent.K2_GetComponentLocation` (`self.Mannequin`)) (`SceneComponent.K2_GetComponentLocation` (`self.Endpoint`)) :`ErrorTolerance` 0.1)
      (`self.K2_DestroyActor`))))

(fn `UserConstructionScript`)