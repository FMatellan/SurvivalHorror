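; BP_Interaction_LightSwitch is an interactable light switch actor that turns a referenced light on and off.
; Its Interact event checks that the Light reference is valid, then flips the visibility of that light's LightComponent without propagating to children.
; It has no other active logic, as the construction script only calls its parent.
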(event `/Game/GameBP/Interfaces/BPI_Interaction.Interact`
  (bind _light (`self.Light`))
  (bind _lightcomponent (`Light.LightComponent` _light))
  (`/Engine/EditorBlueprintResources/StandardMacros.IsValid` _light
    (:`Is Valid`
      (if (`SceneComponent.IsVisible` _lightcomponent)
        (`SceneComponent.SetVisibility` _lightcomponent false false)
        (else
          (`SceneComponent.SetVisibility` _lightcomponent true false))))))

(fn `UserConstructionScript`
  (`parent.UserConstructionScript`))