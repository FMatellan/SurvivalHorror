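; Actor component that gives BP_Character a Tetris-style grid inventory with stacking, rotation, healing item use, dropping and examination.
; Items are stored by grid cell, while a parallel occupancy map tracks cells covered by each rotated data-asset shape.
; Pickups top up existing stacks, then try four rotations for free space, reporting any remainder.
; It also creates the inventory and examination widgets, switching movement, look and input mode on toggle.
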(event `self.ReceiveBeginPlay`
  ;[1 1 1] Initialize
  (bind _asbp_character (cast `/Game/Blueprints/BP_Character` (`self.GetOwner`)))
  ;;[1 0.06771 0.06771] Examination Widget
  (set `self.PlayerRef` _asbp_character)
  (bind _returnvalue (`|CreateWidget` "/Game/UMG/Inventory/W_Examination.W_Examination_C" null self))
  (set `self.ExaminationWidgetRef` _returnvalue)
  (set `/Game/Blueprints/Core/PC_HorrorGame.W_ExaminationRef` (`self.ExaminationWidgetRef`) (cast `/Game/Blueprints/Core/PC_HorrorGame` (`GameplayStatics.GetPlayerController` 0) :!pure true))
  (bind _outactors (`GameplayStatics.GetAllActorsOfClass` "/Game/Blueprints/Actors/Inventory/BP_Examination.BP_Examination_C"))
  (set `self.BPExaminationRef` (`|GetArrayItem` _outactors))
  (set `/Game/UMG/Inventory/W_Examination.AC_Inventory_Ref` self (`self.ExaminationWidgetRef`))
  (`self.DefaultInventoryState`)
  (bind _returnvalue_2 (`|CreateWidget` "/Game/TetrisInventory/Widgets/W_Inventory.W_Inventory_C" null (`self.Inventory`) (`self.InventorySize`) (`self.InventoryWidth`) self))
  (bind _output_get (set `self.W_Inventory_Ref` _returnvalue_2))
  (`UserWidget.AddToViewport` _output_get 0)
  (`Widget.SetVisibility` _output_get "Hidden"))

(event `ToggleInventory`
  (bind _returnvalue (`GameplayStatics.GetPlayerController` 0))
  (bind _examinationwidgetref (`self.ExaminationWidgetRef`))
  (bind _w_inventory_ref (`self.W_Inventory_Ref`))
  (bind _charactermovement (`Character.CharacterMovement` (`self.PlayerRef`)))
  ;[1 1 1] Toggle
  (if (`self.CanOpenInventory`)
    (if (`self.InventoryOpen`)
      (set `self.InventoryOpen` false)
      (`CharacterMovementComponent.SetMovementMode` _charactermovement "MOVE_Walking" 0)
      (`Controller.ResetIgnoreLookInput` _returnvalue)
      (set `PlayerController.bShowMouseCursor` false _returnvalue)
      (`Widget.SetVisibility` _w_inventory_ref "Collapsed")
      (`WidgetBlueprintLibrary.SetInputMode_GameOnly` (`GameplayStatics.GetPlayerController` 0))
      (else
        (set `self.InventoryOpen` true)
        (`CharacterMovementComponent.DisableMovement` _charactermovement)
        (`Controller.SetIgnoreLookInput` _returnvalue true)
        (set `PlayerController.bShowMouseCursor` true _returnvalue)
        (`Widget.SetVisibility` _w_inventory_ref "Visible")
        (if (`Widget.IsInViewport` _examinationwidgetref)
          (`self.ResetExaminationItemTransform`)
          (`Widget.RemoveFromParent` _examinationwidgetref))
        (`WidgetBlueprintLibrary.SetInputMode_GameAndUIEx` (`GameplayStatics.GetPlayerController` 0) (`self.W_Inventory_Ref`))
        (`/Game/TetrisInventory/Widgets/W_Inventory.UpdateInventory` (`self.W_Inventory_Ref`) (`self.Inventory`) (`self.InventorySize`) (`self.InventoryWidth`))))))

(event `EnhancedInput|/Game/ThirdPerson/Input/Actions/IA_ToggleInventory`
  (params (ActionValue :type Boolean) (ElapsedSeconds :type "Float (double-precision)") (TriggeredSeconds :type "Float (double-precision)") (InputAction :type "InputAction Object Reference" :default "/Game/ThirdPerson/Input/Actions/IA_ToggleInventory.IA_ToggleInventory"))
  ;[1 1 1] Toggle
  (:`Completed`
    (`self.ToggleInventory`)))

(fn `AddItemFromFloor`
  (params (ItemStructure :type "/Game/TetrisInventory/DataAssets/S_Item Structure"))
  (returns (Success :type Boolean) (Remainig :type Integer))
  (locals (`L-ItemStructure` :type "/Game/TetrisInventory/DataAssets/S_Item Structure") (`L-LoopKey` :type "Vector2D Structure") (`L-LoopValue` :type "/Game/TetrisInventory/DataAssets/S_Item Structure"))
  (bind ((`DataAsset_39_AC02AB6E4681C9C9EB62F3B66DE3B5AC` _dataasset) (`Rotation_6_3CFA842B4A637286AF03A095E755EF4E` _rotation) (`Quantity_8_3CC32AE94EA81BDD63199E92D5C65573` _quantity)) (break `/Game/TetrisInventory/DataAssets/S_Item` (`local.L-LoopValue`)))
  (bind (_returnvalue _remaining) (`self.IsNotFullyStacked` (`local.L-LoopValue`)))
  (set `local.L-ItemStructure` ItemStructure)
  (`|ExecutionSequence`
    (:`then_0`
      (bind _keys (`BlueprintMapLibrary.Map_Keys` (`self.Inventory`)))
      (for _array_element _keys
        (bind _output_get (set `local.L-LoopKey` _array_element))
        (set `local.L-LoopValue` (`BlueprintMapLibrary.Map_Find` (`self.Inventory`) _output_get))
        (if (== (`.DataAsset_39_AC02AB6E4681C9C9EB62F3B66DE3B5AC` (break `/Game/TetrisInventory/DataAssets/S_Item` (`local.L-ItemStructure`))) (`.DataAsset_39_AC02AB6E4681C9C9EB62F3B66DE3B5AC` (break `/Game/TetrisInventory/DataAssets/S_Item` (`local.L-LoopValue`))))
          (if _returnvalue
            (`self.AddToInventory` (`local.L-LoopKey`) (make `/Game/TetrisInventory/DataAssets/S_Item` :`Data Asset` _dataasset :`Rotation` _rotation :`Quantity` (`KismetMathLibrary.Clamp` (+ _quantity (`.Quantity_8_3CC32AE94EA81BDD63199E92D5C65573` (break `/Game/TetrisInventory/DataAssets/S_Item` (`local.L-ItemStructure`)))) 0 (`/Game/TetrisInventory/DataAssets/ParentAssets/DA_Items.MaxQuantity` _dataasset))))
            (bind _structout (setmembers `/Game/TetrisInventory/DataAssets/S_Item` :`StructRef` (`local.L-ItemStructure`) :`Quantity` (- (`.Quantity_8_3CC32AE94EA81BDD63199E92D5C65573` (break `/Game/TetrisInventory/DataAssets/S_Item` (`local.L-ItemStructure`))) _remaining)))
            (if (<= (`.Quantity_8_3CC32AE94EA81BDD63199E92D5C65573` (break `/Game/TetrisInventory/DataAssets/S_Item` _structout)) 0)
              (return true 0))))))
    (:`then_1`
      (`|ExecutionSequence`
        (:`then_0`
          (bind _success (`self.CheckRotationFit` (`local.L-ItemStructure`)))
          (if _success
            (return true 0)))
        (:`then_1`
          (bind _success_2 (`self.CheckRotationFit` (`local.L-ItemStructure`) 90.0))
          (if _success_2
            (return true 0)))
        (:`then_2`
          (bind _success_3 (`self.CheckRotationFit` (`local.L-ItemStructure`) 180.0))
          (if _success_3
            (return true 0)))
        (:`then_3`
          (bind _success_4 (`self.CheckRotationFit` (`local.L-ItemStructure`) -90.0))
          (if _success_4
            (return true 0)))
        (:`then_4`
          (return false (`.Quantity_8_3CC32AE94EA81BDD63199E92D5C65573` (break `/Game/TetrisInventory/DataAssets/S_Item` (`local.L-ItemStructure`)))))))))

(fn `AddToInventory`
  (params (Key :type "Vector2D Structure") (Value :type "/Game/TetrisInventory/DataAssets/S_Item Structure") (ModifyState :type Boolean))
  (`BlueprintMapLibrary.Map_Add` (`self.Inventory`) Key Value)
  (if (`local.ModifyState`)
    (`self.AddToState` (`local.Value`) (`local.Key`))))

(fn `AddToState`
  (params (S_Item :type "/Game/TetrisInventory/DataAssets/S_Item Structure") (Location :type "Vector2D Structure"))
  (bind (_dataasset _rotation) (break `/Game/TetrisInventory/DataAssets/S_Item` S_Item))
  (for _array_element (`/Game/TetrisInventory/DataAssets/ParentAssets/DA_Items.GetShape` _dataasset _rotation)
    (`BlueprintMapLibrary.Map_Add` (`self.InventoryState`) (+ _array_element Location) true)))

(fn `CheckRotationFit`
  (params (Structure :type "/Game/TetrisInventory/DataAssets/S_Item Structure") (Rotation :type "Float (double-precision)"))
  (returns (Success :type Boolean))
  (bind (_dataasset _rotation _quantity) (break `/Game/TetrisInventory/DataAssets/S_Item` Structure))
  (bind (_returnvalue _validkey) (`self.WhereShapeFits` (`/Game/TetrisInventory/DataAssets/ParentAssets/DA_Items.GetShape` (`.DataAsset_39_AC02AB6E4681C9C9EB62F3B66DE3B5AC` (break `/Game/TetrisInventory/DataAssets/S_Item` Structure)) Rotation)))
  (if _returnvalue
    (`self.AddToInventory` _validkey (make `/Game/TetrisInventory/DataAssets/S_Item` _dataasset Rotation _quantity) true)
    (return true)
    (else
      (return false))))

(fn `Create Examination Widget`
  (params (Key :type "Vector2D Structure"))
  (bind _examinationwidgetref (`self.ExaminationWidgetRef`))
  (`/Game/UMG/Inventory/W_Examination.UpdateWidget` _examinationwidgetref (`BlueprintMapLibrary.Map_Find` (`self.Inventory`) Key))
  (`Widget.SetVisibility` (`self.W_Inventory_Ref`) "Collapsed")
  (`UserWidget.AddToViewport` _examinationwidgetref 3)
  (set `self.CanOpenInventory` false))

(fn `DefaultInventoryState`
  (locals (GridX :type "Float (double-precision)") (GridY :type "Float (double-precision)"))
  (for _ (range (`self.InventorySize`))
    (`BlueprintMapLibrary.Map_Add` (`self.InventoryState`) (`KismetMathLibrary.MakeVector2D` (`local.GridX`) (`local.GridY`)))
    (if (== (`local.GridX`) (- (`self.InventoryWidth`) 1))
      (set `local.GridX` 0.0)
      (`/Engine/EditorBlueprintResources/StandardMacros.IncrementFloat` (`local.GridY`))
      (else
        (`/Engine/EditorBlueprintResources/StandardMacros.IncrementFloat` (`local.GridX`)))))
  (bind _keys (`BlueprintMapLibrary.Map_Keys` (`self.Inventory`)))
  (for _array_element _keys
    (`self.AddToState` (`BlueprintMapLibrary.Map_Find` (`self.Inventory`) _array_element) _array_element)))

(fn `DropItem`
  (params (Structure :type "/Game/TetrisInventory/DataAssets/S_Item Structure"))
  (bind _returnvalue (`self.GetOwner`))
  (bind _returnvalue_2 (+ (`Actor.K2_GetActorLocation` _returnvalue) (* (`Actor.GetActorForwardVector` _returnvalue) 600.0)))
  (bind (_outhit _returnvalue_3) (`KismetSystemLibrary.LineTraceSingle` _returnvalue_2 (- _returnvalue_2 (0.0 0.0 500.0)) "TraceTypeQuery1"))
  (if _returnvalue_3
    (`|SpawnActorFromClass` "/Game/TetrisInventory/BP_Item.BP_Item_C" (`KismetMathLibrary.MakeTransform` (`.ImpactPoint` (`GameplayStatics.BreakHitResult` _outhit))) "Undefined" "MultiplyWithRoot" null (`local.Structure`) null)))

(fn `IsNotFullyStacked`
  (params (ItemStructure :type "/Game/TetrisInventory/DataAssets/S_Item Structure"))
  (returns (ReturnValue :type Boolean) (Remaining :type Integer))
  (bind ((`DataAsset_39_AC02AB6E4681C9C9EB62F3B66DE3B5AC` _dataasset) (`Quantity_8_3CC32AE94EA81BDD63199E92D5C65573` _quantity)) (break `/Game/TetrisInventory/DataAssets/S_Item` ItemStructure))
  (bind _maxquantity (`/Game/TetrisInventory/DataAssets/ParentAssets/DA_Items.MaxQuantity` _dataasset))
  (return (> _maxquantity _quantity) (- _maxquantity _quantity)))

(fn `PickUpItem`
  (params (ItemRef :type "/Game/TetrisInventory/BP_Item Object Reference"))
  (returns (ReturnValue :type Boolean))
  (bind (_success _remainig) (`self.AddItemFromFloor` (`/Game/TetrisInventory/BP_Item.ItemStructure` ItemRef)))
  (if (== _remainig 0)
    (return true)
    (else
      (`/Game/TetrisInventory/BP_Item.ModifyQuantity` (`local.ItemRef`) _remainig)
      (return false))))

(fn `RemoveFromInventory`
  (params (Key :type "Vector2D Structure") (ModifyState :type Boolean))
  (`|ExecutionSequence`
    (:`then_0`
      (if (`local.ModifyState`)
        (`self.RemoveFromState` (`BlueprintMapLibrary.Map_Find` (`self.Inventory`) (`local.Key`)) (`local.Key`))))
    (:`then_1`
      (`BlueprintMapLibrary.Map_Remove` (`self.Inventory`) (`local.Key`)))))

(fn `RemoveFromState`
  (params (S_Item :type "/Game/TetrisInventory/DataAssets/S_Item Structure") (Location :type "Vector2D Structure"))
  (bind (_dataasset _rotation) (break `/Game/TetrisInventory/DataAssets/S_Item` S_Item))
  (for _array_element (`/Game/TetrisInventory/DataAssets/ParentAssets/DA_Items.GetShape` _dataasset _rotation)
    (`BlueprintMapLibrary.Map_Add` (`self.InventoryState`) (+ _array_element Location))))

(fn `ResetExaminationItemTransform`
  (`SceneComponent.K2_SetRelativeLocation` (`/Game/Blueprints/Actors/Inventory/BP_Examination.ItemMesh` (`self.BPExaminationRef`)) (0.0 0.0 0.0) false false))

(fn `UseItem`
  (params (Key :type "Vector2D Structure"))
  (bind (_dataasset _rotation _quantity) (break `/Game/TetrisInventory/DataAssets/S_Item` (`BlueprintMapLibrary.Map_Find` (`self.Inventory`) Key)))
  (switch `/Game/TetrisInventory/DataAssets/E_ItemType` (`/Game/TetrisInventory/DataAssets/ParentAssets/DA_Items.ItemType` _dataasset)
    (:`NewEnumerator0`
      (bind _asda_healing_item (cast `/Game/TetrisInventory/DataAssets/ParentAssets/DA_HealingItem` _dataasset))
      (`/Game/TetrisInventory/DataAssets/ParentAssets/DA_HealingItem.HealPlayer` _asda_healing_item (`self.PlayerRef`))
      (if (> _quantity 0)
        (`/Engine/EditorBlueprintResources/StandardMacros.DecrementInt` _quantity)))))

(fn `WhereShapeFits`
  (params (Shape :type "Array of Vector2D Structure"))
  (returns (ReturnValue :type Boolean) (ValidKey :type "Vector2D Structure"))
  (locals (`L-EmptySlot` :type "Vector2D Structure") (`L-Failed` :type Boolean))
  (bind _keys (`BlueprintMapLibrary.Map_Keys` (`self.InventoryState`)))
  (for _array_element _keys
    (bind (_value _returnvalue) (`BlueprintMapLibrary.Map_Find` (`self.InventoryState`) (- _array_element (`|GetArrayItem` (`local.Shape`)))))
    (if _returnvalue
      (if (not _value)
        (set `local.L-EmptySlot` _array_element)
        (for _array_element_2 (`local.Shape`)
          (bind (_value_2 _returnvalue_2) (`BlueprintMapLibrary.Map_Find` (`self.InventoryState`) (+ (`local.L-EmptySlot`) _array_element_2)))
          (if (or _value_2 (not _returnvalue_2))
            (set `local.L-Failed` true)
            (break)))
        (if (`local.L-Failed`)
          (set `local.L-Failed` false)
          (else
            (return true (`local.L-EmptySlot`)))))))
  (return false (0.0 0.0)))