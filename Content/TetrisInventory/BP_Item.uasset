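; BP_Item is an item actor for the Tetris-style inventory, carrying its data in an item structure.
; On BeginPlay it caches the player character as BP_Character, and ModifyQuantity writes a new quantity into the structure.
; An unconnected pickup chain, which never runs, would pass the item to AC_Inventory, then destroy it on success or print a failure message.
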(event `self.ReceiveBeginPlay`
  (bind _asbp_character (cast `/Game/Blueprints/BP_Character` (`GameplayStatics.GetPlayerCharacter` 0)))
  (set `self.PlayerRef` _asbp_character))

(fn `ModifyQuantity`
  (params (Quantity :type Integer))
  (setmembers `/Game/TetrisInventory/DataAssets/S_Item` :`StructRef` (`self.ItemStructure`) :`Quantity` Quantity))

(fn `UserConstructionScript`)