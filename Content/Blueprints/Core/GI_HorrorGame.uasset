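; Game instance for a horror game that tracks play time, saved chapter and deaths, and handles saving and loading them by slot name.
; A looping one-second timer started on Init increments GameTime and broadcasts OnTimeUpdated.
; SaveGame writes the slot's BP_SaveGame, then records a summary in a shared "MetaSave" index keyed by slot name, creating either object if missing.
; LoadGame restores the values, and a helper formats time as hours and minutes.
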(event `self.ReceiveInit`
  (`KismetSystemLibrary.K2_SetTimerDelegate` (delegate `AddGameTime`) 1.0 true)
  (bind _asbp_character (cast `/Game/Blueprints/BP_Character` (`GameplayStatics.GetPlayerCharacter` 0)))
  (set `/Game/Blueprints/Core/BP_SaveGame.Deaths` (`/Game/Blueprints/BP_Character.PlayerDeaths` _asbp_character) (`self.Savear`)))

(event `AddGameTime`
  (bind _result (`/Engine/EditorBlueprintResources/StandardMacros.IncrementInt` (`self.GameTime`))
    (:`  `
      (`self.OnTimeUpdated` _result))))

(event `SaveGame`
  (params (SaveGameName :type String))
  (bind _savear (`self.Savear`))
  ;[1 1 1] SaveGame
  (bind _returnvalue (`GameplayStatics.DoesSaveGameExist` SaveGameName))
  (if _returnvalue
    (bind _returnvalue_2 (`GameplayStatics.LoadGameFromSlot` SaveGameName))
    (bind _asbp_save_game (cast `/Game/Blueprints/Core/BP_SaveGame` _returnvalue_2))
    (set `self.Savear` _asbp_save_game)
    (else
      (bind _returnvalue_3 (`GameplayStatics.CreateSaveGameObject` "/Game/Blueprints/Core/BP_SaveGame.BP_SaveGame_C"))
      (set `self.Savear` _returnvalue_3)))
  (set `/Game/Blueprints/Core/BP_SaveGame.GameTime` (`self.GameTime`) _savear)
  (set `/Game/Blueprints/Core/BP_SaveGame.ChapterSaved` (`self.ChapterSaved`) _savear)
  (set `/Game/Blueprints/Core/BP_SaveGame.Deaths` (`self.Deaths`) _savear)
  (`GameplayStatics.SaveGameToSlot` (`self.Savear`) SaveGameName)
  (bind _returnvalue_4 (`GameplayStatics.DoesSaveGameExist` "MetaSave"))
  (if _returnvalue_4
    (bind _returnvalue_5 (`GameplayStatics.LoadGameFromSlot` "MetaSave"))
    (bind _asbp_meta_save (cast `/Game/Blueprints/Core/BP_MetaSave` _returnvalue_5))
    (set `self.MetaSave` _asbp_meta_save)
    (else
      (bind _returnvalue_6 (`GameplayStatics.CreateSaveGameObject` "/Game/Blueprints/Core/BP_MetaSave.BP_MetaSave_C"))
      (set `self.MetaSave` _returnvalue_6)))
  (`BlueprintMapLibrary.Map_Add` (`/Game/Blueprints/Core/BP_MetaSave.SaveFiles` (`self.MetaSave`)) SaveGameName (make `/Game/Blueprints/Structs/S_SaveGameMetaData` (`self.GameTime`) (`self.ChapterSaved`) (`self.Deaths`)))
  (`GameplayStatics.SaveGameToSlot` (`self.MetaSave`) "MetaSave"))

(event `LoadGame`
  (params (SaveGameName :type String))
  ;[1 1 1] LoadGame
  (bind _returnvalue (`GameplayStatics.DoesSaveGameExist` SaveGameName))
  (if _returnvalue
    (bind _returnvalue_2 (`GameplayStatics.LoadGameFromSlot` SaveGameName))
    (bind _asbp_save_game (cast `/Game/Blueprints/Core/BP_SaveGame` _returnvalue_2))
    (bind _output_get (set `self.Savear` _asbp_save_game))
    (set `self.GameTime` (`/Game/Blueprints/Core/BP_SaveGame.GameTime` _output_get))
    (set `self.ChapterSaved` (`/Game/Blueprints/Core/BP_SaveGame.ChapterSaved` _output_get))
    (set `self.Deaths` (`/Game/Blueprints/Core/BP_SaveGame.Deaths` _output_get))))

(fn `Get GameTime String`
  (params (GameTime :type Integer))
  (returns (`HoursH MinutesM` :type String))
  (return (`KismetStringLibrary.Concat_StrStr` (`KismetTextLibrary.Conv_TextToString` (`KismetTextLibrary.Conv_IntToText` (/ GameTime 3600) false true 2)) "h " (`KismetTextLibrary.Conv_TextToString` (`KismetTextLibrary.Conv_IntToText` (/ (mod GameTime 3600) 60) false true 2)) "m")))