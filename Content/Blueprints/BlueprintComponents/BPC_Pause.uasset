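; BPC_Pause is a Blueprint component that pauses the game and handles the pause menu widget.
; On BeginPlay it creates W_PauseMenu and adds it to the viewport collapsed.
; IA_Pause removes all widgets, sets the stored menu visible without re-adding it, focuses it in Game and UI input mode, shows the cursor and pauses.
; It contains no unpause logic.
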(event `self.ReceiveBeginPlay`
  (bind _returnvalue (`|CreateWidget` "/Game/UMG/Pause/W_PauseMenu.W_PauseMenu_C"))
  (bind _output_get (set `self.PauseMenu Widget` _returnvalue))
  (`UserWidget.AddToViewport` _output_get 0)
  (`Widget.SetVisibility` (`self.PauseMenu Widget`) "Collapsed"))

(event `EnhancedInput|/Game/ThirdPerson/Input/Actions/IA_Pause`
  (params (ActionValue :type Boolean) (ElapsedSeconds :type "Float (double-precision)") (TriggeredSeconds :type "Float (double-precision)") (InputAction :type "InputAction Object Reference" :default "/Game/ThirdPerson/Input/Actions/IA_Pause.IA_Pause"))
  (:`Triggered`
    (`WidgetLayoutLibrary.RemoveAllWidgets`)
    (`Widget.SetVisibility` (`self.PauseMenu Widget`) "Visible")
    (`WidgetBlueprintLibrary.SetInputMode_GameAndUIEx` (`GameplayStatics.GetPlayerController` 0) (`self.PauseMenu Widget`))
    (set `PlayerController.bShowMouseCursor` true (`GameplayStatics.GetPlayerController` 0))
    (`GameplayStatics.SetGamePaused` true)))