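; BPC_Health is a health component that tracks current health and drives a blood screen effect.
; AddHealth and RemoveHealth change CurrentHealth, clamped between the minimum and maximum, then refresh the effect, which is also updated on BeginPlay.
; UpdateBloodScreen maps health onto the Radius scalar in the MPC_Bloodscreen material parameter collection, so the screen effect follows health without a direct material reference.
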(event `self.ReceiveBeginPlay`
  (`self.UpdateBloodScreen`))

(fn `AddHealth`
  (params (Amount :type "Float (double-precision)"))
  (set `self.CurrentHealth` (`KismetMathLibrary.FClamp` (+ Amount (`self.CurrentHealth`)) (`self.MinHeatlh`) (`self.MaxHealth`)))
  (`self.UpdateBloodScreen`))

(fn `RemoveHealth`
  (params (Amount :type "Float (double-precision)"))
  (set `self.CurrentHealth` (`KismetMathLibrary.FClamp` (- (`self.CurrentHealth`) Amount) (`self.MinHeatlh`) (`self.MaxHealth`)))
  (`self.UpdateBloodScreen`))

(fn `UpdateBloodScreen`
  (`KismetMaterialLibrary.SetScalarParameterValue` "/Game/Props/Materials/MPC_Bloodscreen.MPC_Bloodscreen" "Radius" (`KismetMathLibrary.MapRangeClamped` (`self.CurrentHealth`) (`self.MinHeatlh`) (`self.MaxHealth`) 0.5 1.0)))