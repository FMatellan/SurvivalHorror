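; BP_HideActor is an interactable hiding spot that moves the player character into or out of hiding.
; Interact starts a looping per-frame timer that interpolates the player at constant speed toward HidingPosition or ExitPosition, chosen by the player's IsHiding flag.
; Entering disables collision, movement and inventory access; completing an exit restores them.
; On arrival it clears the timers, fires a finished-moving dispatcher and toggles IsHiding.
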(event `self.ReceiveBeginPlay`
  (bind _asbp_character (cast `/Game/Blueprints/BP_Character` (`GameplayStatics.GetPlayerCharacter` 0)))
  (set `self.PlayerRef` _asbp_character)
  (bind _aspc_horror_game (cast `/Game/Blueprints/Core/PC_HorrorGame` (`GameplayStatics.GetPlayerController` 0)))
  (set `self.ControllerRef` _aspc_horror_game))

(event `/Game/Blueprints/Interfaces/BPI_Interaction.Interact`
  (bind _playerref (`self.PlayerRef`))
  (if (`/Game/Blueprints/BP_Character.IsHiding` _playerref)
    (bind _returnvalue (`KismetSystemLibrary.K2_SetTimerDelegate` (delegate `MoveCharacter`) (`GameplayStatics.GetWorldDeltaSeconds`) true))
    (else
      (`self.SetActorEnableCollision` _playerref false)
      (`CharacterMovementComponent.DisableMovement` (`Character.CharacterMovement` _playerref))
      (set `/Game/Blueprints/Core/PC_HorrorGame.CanOpenInventory` false (`self.ControllerRef`))
      (bind _returnvalue_2 (`KismetSystemLibrary.K2_SetTimerDelegate` (delegate `MoveCharacter`) (`GameplayStatics.GetWorldDeltaSeconds`) true)))))

(event `MoveCharacter`
  (bind _playerref (`self.PlayerRef`))
  (`self.K2_SetActorTransform` _playerref (`KismetMathLibrary.MakeTransform` (`KismetMathLibrary.VInterpTo_Constant` (`self.K2_GetActorLocation` _playerref) (`SceneComponent.K2_GetComponentLocation` (select `bool` (`/Game/Blueprints/BP_Character.IsHiding` (`self.PlayerRef`)) :`false` (`self.HidingPosition`) :`true` (`self.ExitPosition`) :!type "SceneComponent Object Reference")) (`GameplayStatics.GetWorldDeltaSeconds`) 1000.0)) false false)
  (if (== (`self.K2_GetActorLocation` (`self.PlayerRef`)) (`SceneComponent.K2_GetComponentLocation` (select `bool` (`/Game/Blueprints/BP_Character.IsHiding` (`self.PlayerRef`)) :`false` (`self.HidingPosition`) :`true` (`self.ExitPosition`))) :`ErrorTolerance` 0.01)
    (`KismetSystemLibrary.K2_ClearAndInvalidateTimerHandle` (stale `/Game/Blueprints/Interfaces/BPI_Interaction.Interact` _returnvalue_2))
    (`KismetSystemLibrary.K2_ClearAndInvalidateTimerHandle` (stale `/Game/Blueprints/Interfaces/BPI_Interaction.Interact` _returnvalue))
    (`self.FinishedMoving`)))

(event `FinishedMoving`
  (bind _playerref (`self.PlayerRef`))
  (bind _playerref_2 (`self.PlayerRef`))
  (`self.FinishedMovingED`)
  (if (`/Game/Blueprints/BP_Character.IsHiding` _playerref)
    (set `/Game/Blueprints/BP_Character.IsHiding` false _playerref)
    (`self.SetActorEnableCollision` _playerref_2 true)
    (`CharacterMovementComponent.SetMovementMode` (`Character.CharacterMovement` _playerref_2) "MOVE_Walking" 0)
    (set `/Game/Blueprints/Core/PC_HorrorGame.CanOpenInventory` true (`self.ControllerRef`))
    (else
      (set `/Game/Blueprints/BP_Character.IsHiding` true _playerref))))

(fn `UserConstructionScript`)