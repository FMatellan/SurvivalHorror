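; Base note actor that the player can approach and examine, with configurable front and back text set in the construction script.
; An overlap sphere starts per-tick visibility traces to the player, showing a camera-facing prompt above the paper when unobstructed.
; Within pickup distance, the prompt toggles and input is enabled.
; The action input creates a W_NoteExamination widget, passing it the note and the level's BP_NoteExamination actor.
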(event `self.ReceiveBeginPlay`
  (bind _outactors (`GameplayStatics.GetAllActorsOfClass` "/Game/Blueprints/Actors/Notes/BP_NoteExamination.BP_NoteExamination_C"))
  (set `self.BPNoteExaminationRef` (`|GetArrayItem` _outactors)))

(event `self.OverlapSphere.OnComponentBeginOverlap`
  (params (OverlappedComponent :type "PrimitiveComponent Object Reference") (OtherActor :type "Actor Object Reference") (OtherComp :type "PrimitiveComponent Object Reference") (OtherBodyIndex :type Integer) (bFromSweep :type Boolean) (SweepResult :type "HitResult Structure (by ref)"))
  (bind _asbp_character (cast `/Game/Blueprints/BP_Character` OtherActor))
  (set `self.PlayerRef` _asbp_character)
  (`SceneComponent.SetVisibility` (`self.PromptWidget`) true false)
  (set `self.UpdateActor` true))

(event `self.OverlapSphere.OnComponentEndOverlap`
  (params (OverlappedComponent :type "PrimitiveComponent Object Reference") (OtherActor :type "Actor Object Reference") (OtherComp :type "PrimitiveComponent Object Reference") (OtherBodyIndex :type Integer))
  (cast `/Game/Blueprints/BP_Character` OtherActor)
  (`SceneComponent.SetVisibility` (`self.PromptWidget`) false false)
  (set `self.UpdateActor` false)
  (`self.DisableInput` (`GameplayStatics.GetPlayerController` 0)))

(event `self.ReceiveTick`
  (params (DeltaSeconds :type "Float (single-precision)"))
  (bind _returnvalue (`GameplayStatics.GetPlayerController` 0))
  (bind _promptwidget (`self.PromptWidget`))
  (bind (_returnvalue_x _returnvalue_y _returnvalue_z) (`KismetMathLibrary.BreakVector` (`SceneComponent.K2_GetComponentLocation` (`self.PaperMesh`))))
  (`SceneComponent.K2_SetWorldLocation` (`self.PromptWidget`) (`KismetMathLibrary.MakeVector` _returnvalue_x _returnvalue_y (+ _returnvalue_z (`self.WidgetDistanceAboveMesh`))) false false)
  (if (`self.UpdateActor`)
    (bind (_outhit _returnvalue_2) (`KismetSystemLibrary.LineTraceSingle` (`self.K2_GetActorLocation`) (`self.K2_GetActorLocation` (`self.PlayerRef`)) "TraceTypeQuery1"))
    (if (not _returnvalue_2)
      (`SceneComponent.SetVisibility` _promptwidget true false)
      (`SceneComponent.K2_SetWorldRotation` (`self.PromptWidget`) (`KismetMathLibrary.FindLookAtRotation` (`SceneComponent.K2_GetComponentLocation` (`self.PromptWidget`)) (`SceneComponent.K2_GetComponentLocation` (`/Game/Blueprints/BP_Character.FollowCamera` (`self.PlayerRef`)))) false false)
      (bind (_bblockinghit _binitialoverlap _time _distance _location _impactpoint _normal _impactnormal _physmat _hitactor _hitcomponent _hitbonename _bonename _hititem _elementindex _faceindex _tracestart _traceend) (`GameplayStatics.BreakHitResult` _outhit))
      (bind _returnvalue_3 (<= (`KismetMathLibrary.VSize` (- _tracestart _traceend)) (`self.PickupDistance`)))
      (`/Game/UMG/Inventory/W_PickUpPrompt.TogglePrompt` (cast `/Game/UMG/Inventory/W_PickUpPrompt` (`WidgetComponent.GetUserWidgetObject` (`self.PromptWidget`)) :!pure true) _returnvalue_3)
      (if _returnvalue_3
        (`self.EnableInput` _returnvalue)
        (else
          (`self.DisableInput` _returnvalue)))
      (else
        (`SceneComponent.SetVisibility` _promptwidget false false)
        (`self.DisableInput` (`GameplayStatics.GetPlayerController` 0))))))

(event `EnhancedInput|/Game/ThirdPerson/Input/Actions/IA_Action`
  (params (ActionValue :type Boolean) (ElapsedSeconds :type "Float (double-precision)") (TriggeredSeconds :type "Float (double-precision)") (InputAction :type "InputAction Object Reference" :default "/Game/ThirdPerson/Input/Actions/IA_Action.IA_Action"))
  (:`Completed`
    (`/Engine/EditorBlueprintResources/StandardMacros.IsValid` (`self.WExaminationNoteRef`)
      (:`Is Not Valid`
        (bind _returnvalue (`|CreateWidget` "/Game/UMG/W_NoteExamination.W_NoteExamination_C" null (`self.BPNoteExaminationRef`)))
        (bind _output_get (set `self.WExaminationNoteRef` _returnvalue))
        (`/Game/UMG/W_NoteExamination.UpdateWidget` _output_get self)
        (`UserWidget.AddToViewport` _output_get 0)))))

(fn `UserConstructionScript`
  (`TextRenderComponent.K2_SetText` (`self.NoteText`) (`self.NoteText(Text)`))
  (`TextRenderComponent.K2_SetText` (`self.BackNoteText`) (`self.BackNoteText(Text)`)))