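; Security camera console that lets the player view and cycle through all BP_SecurityCamera actors in the level.
; Interact toggles viewing, swapping player input and HUD for the controller's input and blending the view target to the current camera.
; Space bar advances to the next camera with wraparound, and IA_Action exits back to the character.
; A timeline started at BeginPlay drives only the current camera's yaw, reversing after a short pause.
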(event `self.ReceiveBeginPlay`
  (bind _outactors (`GameplayStatics.GetAllActorsOfClass` "/Game/Blueprints/Actors/SecurityCameras/BP_SecurityCamera.BP_SecurityCamera_C"))
  (set `self.SecurityCameras` _outactors)
  (bind (_direction _alpha) (`Timeline|RotateCamera` :!label _label)
    (:`Update`
      (`SceneComponent.K2_SetRelativeRotation` (`/Game/Blueprints/Actors/SecurityCameras/BP_SecurityCamera.Camera` (`|GetArrayItem` (`self.SecurityCameras`) (`self.CurrentCameraIndex`))) (`KismetMathLibrary.MakeRotator` 0.0 0.0 _alpha) false false))
    (:`Finished`
      (`KismetSystemLibrary.Delay` 0.2)
      (goto _label :!via `Reverse`))))

(event `/Game/Blueprints/Interfaces/BPI_Interaction.Interact`
  (bind _returnvalue (`GameplayStatics.GetPlayerCharacter` 0))
  (bind _returnvalue_2 (`GameplayStatics.GetPlayerController` 0))
  (if (`self.isViewingCameras`)
    (`self.LeaveCameraController`)
    (else
      (set `self.isViewingCameras` true)
      (`self.DisableInput` _returnvalue _returnvalue_2)
      (`Controller.SetIgnoreLookInput` _returnvalue_2 true)
      (`Widget.SetVisibility` (`/Game/Blueprints/BP_Character.MainHUDRef` (cast `/Game/Blueprints/BP_Character` _returnvalue :!pure true)) "Hidden")
      (`self.EnableInput` (`GameplayStatics.GetPlayerController` 0))
      (`self.ViewThroughCamera`))))

(event `LeaveCameraController`
  (bind _returnvalue (`GameplayStatics.GetPlayerController` 0))
  (bind _returnvalue_2 (`GameplayStatics.GetPlayerCharacter` 0))
  (bind _returnvalue_3 (`GameplayStatics.GetPlayerController` 0))
  (set `self.isViewingCameras` false)
  (`self.DisableInput` _returnvalue)
  (`Controller.ResetIgnoreLookInput` _returnvalue)
  (`Widget.SetVisibility` (`/Game/Blueprints/BP_Character.MainHUDRef` (cast `/Game/Blueprints/BP_Character` (`GameplayStatics.GetPlayerCharacter` 0) :!pure true)) "SelfHitTestInvisible")
  (`self.EnableInput` _returnvalue_2 _returnvalue_3)
  (`PlayerController.SetViewTargetWithBlend` _returnvalue_3 _returnvalue_2 0.0 "VTBlend_Linear" 0.0 false))

(event `Key|SpaceBar`
  (params (Key :type "Key Structure"))
  (bind _returnvalue (+ (`self.CurrentCameraIndex`) 1))
  (:`Pressed`
    (set `self.CurrentCameraIndex` (select `bool` (> _returnvalue (- (`KismetArrayLibrary.Array_Length` (`self.SecurityCameras`)) 1)) :`false` _returnvalue))
    (`self.ViewThroughCamera`)))

(event `InputAction|Return`
  (params (Key :type "Key Structure")))

(event `EnhancedInput|/Game/ThirdPerson/Input/Actions/IA_Action`
  (params (ActionValue :type Boolean) (ElapsedSeconds :type "Float (double-precision)") (TriggeredSeconds :type "Float (double-precision)") (InputAction :type "InputAction Object Reference" :default "/Game/ThirdPerson/Input/Actions/IA_Action.IA_Action"))
  (:`Completed`
    (`self.LeaveCameraController`)))

(fn `UserConstructionScript`)

(fn `ViewThroughCamera`
  (`PlayerController.SetViewTargetWithBlend` (`GameplayStatics.GetPlayerController` 0) (`|GetArrayItem` (`self.SecurityCameras`) (`self.CurrentCameraIndex`)) 0.0 "VTBlend_Linear" 0.0 false)
  (return))